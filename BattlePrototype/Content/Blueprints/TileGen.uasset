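; TileGen is an actor that lays out a flat MaxX by MaxY grid of static mesh tiles, spaced by TileSize.
; Its construction script adds one component per tile in a single loop, using modulo and integer division to derive column and row.
; Two further loops draw long-lived red debug lines, offset half a tile from the mesh origins, to mark tile boundaries.
; The event graph is unused.
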(event EventBeginPlay)

(event Collision|EventActorBeginOverlap
  (params (OtherActor :type Actor%20Object%20Reference)))

(event EventTick
  (params (DeltaSeconds :type Float%20%28single-precision%29)))

(fn ConstructionScript
  (bind _returnvalue (Transformation|GetActorLocation))
  (bind _returnvalue_2 (Transformation|GetActorLocation))
  (bind _maxx (Variables|Default|GetMaxX))
  (bind _tilesize (Variables|Default|GetTileSize))
  (bind _tilesize_2 (Variables|Default|GetTileSize))
  (bind _tilesize_3 (Variables|Default|GetTileSize))
  (bind _returnvalue_3 (/ _tilesize_3 2))
  (bind _returnvalue_4 (/ _tilesize_2 2))
  (for _index (range 0 (- (* (Variables|Default|GetMaxX) (Variables|Default|GetMaxY)) 1))
    (AddComponent|AddStaticMeshComponent false (Math|Transform|MakeTransform (Math|Conversions|ToVector(Float) (Utilities|Struct|MakeIntVector (* (Math|Integer|%(Integer) _index _maxx) _tilesize) (* (/ _index _maxx) _tilesize))) "0, 0, 0" "1.500000,1.500000,1")))
  (for _index_2 (range 1 (- (Variables|Default|GetMaxX) 1))
    (Rendering|Debug|DrawDebugLine (+ (Math|Vector|MakeVector (Math|Conversions|ToFloat(Integer) (- (* _index_2 _tilesize_3) _returnvalue_3)) (Math|Conversions|ToFloat(Integer) (- 0 _returnvalue_3)) 0.0) _returnvalue_2) (+ _returnvalue_2 (Math|Vector|MakeVector (Math|Conversions|ToFloat(Integer) (- (* _index_2 _tilesize_3) _returnvalue_3)) (Math|Conversions|ToFloat(Integer) (- (* (Variables|Default|GetMaxY) _tilesize_3) _returnvalue_3)) 0.0)) "(R=0.871367,G=0.064803,B=0.063010,A=1.000000)" 1e+02 5.0))
  (for _index_3 (range 0 (- (Variables|Default|GetMaxY) 1))
    (Rendering|Debug|DrawDebugLine (+ (Math|Vector|MakeVector (Math|Conversions|ToFloat(Integer) (- 0 _returnvalue_4)) (Math|Conversions|ToFloat(Integer) (- (* _index_3 _tilesize_2) _returnvalue_4)) 0.0) _returnvalue) (+ _returnvalue (Math|Vector|MakeVector (Math|Conversions|ToFloat(Integer) (- (* (Variables|Default|GetMaxX) _tilesize_2) _returnvalue_4)) (Math|Conversions|ToFloat(Integer) (- (* _index_3 _tilesize_2) _returnvalue_4)) 0.0)) "(R=0.871367,G=0.064803,B=0.063010,A=1.000000)" 1e+02 5.0)))